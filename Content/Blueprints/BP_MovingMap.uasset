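; BP_MovingMap is a map segment for a procedurally extended level, with a randomly placed child actor as its shark spawn.
; Construction gathers the shark spawn point transforms and adds one child actor at a random one.
; AttachMaps exposes the NextAttachPoint location as a transform for chaining segments.
; When BP_CharTest overlaps EndTrigger, BP_GameModeBase adds a floor, and this segment destroys itself after a short delay.
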(event OnComponentBeginOverlap(EndTrigger)
  (params (OverlappedComponent :type Primitive%20Component%20Object%20Reference) (OtherActor :type Actor%20Object%20Reference) (OtherComp :type Primitive%20Component%20Object%20Reference) (OtherBodyIndex :type Integer) (bFromSweep :type Boolean) (SweepResult :type Hit%20Result%20Structure%20%28by%20ref%29))
  (Utilities|Casting|CastToBP_CharTest OtherActor)
  (bind _asbp_game_mode_base (Utilities|Casting|CastToBP_GameModeBase (Game|GetGameMode)))
  (Default|AddFloor _asbp_game_mode_base)
  (Utilities|FlowControl|Delay 2.0)
  (Actor|DestroyActor))

(event EventBeginPlay)

(fn ConstructionScript
  (CallFunction|SharkSpawnPoints)
  (CallFunction|SpawnSharks))

(fn AttachMaps
  (return (Math|Conversions|ToTransform(Vector) (Transformation|GetWorldLocation (Variables|Default|GetNextAttachPoint)))))

(fn SharkSpawnPoints
  (Variables|Default|SetSpawnPoints (Utilities|Array|MakeArray (Transformation|GetRelativeTransform (Variables|Default|GetSpawnShark)) (Transformation|GetRelativeTransform (Variables|Default|GetSpawnShark2)) (Transformation|GetRelativeTransform (Variables|Default|GetSpawnShark3)) "")))

(fn SpawnSharks
  (bind _spawnpoints (Variables|Default|GetSpawnPoints))
  (AddComponent|AddChildActorComponent false (Utilities|Array|Get(acopy) _spawnpoints (Math|Random|RandomIntegerinRange 0 (Utilities|Array|LastIndex _spawnpoints)))))